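; BP_Actor_Status_Heal is a character status actor that heals its owning pawn once, when the status begins.
; EventStatusBegin checks that the owning pawn is valid and casts it to BP_Character_CharacterStatus.
; It then passes the negated Value to ApplyDamage with itself as causer, so healing travels through the damage pipeline as negative damage.
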(event EventBeginPlay
  (|CallParentFunction))

(event Collision|EventActorBeginOverlap
  (params (OtherActor :type Actor%20Object%20Reference))
  (|CallParentFunction OtherActor) ; This node is disabled and will not be called.\nDrag off pins to build functionality.
)

(event EventTick
  (params (DeltaSeconds :type Float%20%28single-precision%29))
  (|CallParentFunction DeltaSeconds) ; This node is disabled and will not be called.\nDrag off pins to build functionality.
)

(event EventEventStatusBegin
  (bind _as_owning__pawn (Variables|Default|GetAs%20Owning%20%20Pawn)
    (:then
      (bind _asbp_character_character_status (Utilities|Casting|CastToBP_Character_CharacterStatus _as_owning__pawn))
      (Game|Damage|ApplyDamage _asbp_character_character_status (* (Variables|Default|GetValue) -1.0) 0 self))
    (:else)))

(fn ConstructionScript
  (|CallParentFunction))