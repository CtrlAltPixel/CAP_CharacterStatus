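; HealthGrowth character status actor that enlarges its owning pawn to a fixed uniform scale.
; On status begin, it reads one attribute from the character's attributes component, binds to that component's attribute-update event and calls UpdateScale.
; It then ends the status immediately.
; UpdateScale ignores the attribute passed in, so the scale does not vary with its value.
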(event Custom|UpdateScale
  (params (Attribute :type F%20Attributes%20Structure))
  (Transformation|SetActorScale3D (Variables|Default|GetAs%20Owning%20%20Pawn) "1.500000,1.500000,1.500000"))

(event EventBeginPlay
  (|CallParentFunction) ; This node is disabled and will not be called.\nDrag off pins to build functionality.
)

(event Collision|EventActorBeginOverlap
  (params (OtherActor :type Actor%20Object%20Reference))
  (|CallParentFunction OtherActor) ; This node is disabled and will not be called.\nDrag off pins to build functionality.
)

(event EventTick
  (params (DeltaSeconds :type Float%20%28single-precision%29))
  (|CallParentFunction DeltaSeconds) ; This node is disabled and will not be called.\nDrag off pins to build functionality.
)

(event EventEventStatusBegin
  (|CallParentFunction)
  (bind _as_owning__pawn (Variables|Default|GetAs%20Owning%20%20Pawn)
    (:then
      (bind _asbp_character_character_status (Utilities|Casting|CastToBP_Character_CharacterStatus _as_owning__pawn))
      (Utilities|IsValid (Variables|/Game/CharacterStatuses/Character/BP_Character_CharacterStatus.BP_Character_CharacterStatus_C|GetBP_AC_Attributes _asbp_character_character_status)
        (:Is%20Valid
          (bind _attribute (Default|GetAttribute (Variables|/Game/CharacterStatuses/Character/BP_Character_CharacterStatus.BP_Character_CharacterStatus_C|GetBP_AC_Attributes _asbp_character_character_status) "NewEnumerator0"))
          (EventDispatchers|BindEventtoOnUpdateAttribute (Variables|/Game/CharacterStatuses/Character/BP_Character_CharacterStatus.BP_Character_CharacterStatus_C|GetBP_AC_Attributes _asbp_character_character_status) (EventDispatchers|CreateEvent :!event Custom|UpdateScale))
          (CallFunction|UpdateScale _attribute)
          (CallFunction|EventStatusEnd))))
    (:else)))

(fn ConstructionScript
  (|CallParentFunction))