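; BP_Actor_Status is an Actor for a turn-based character status effect, apparently a base with an empty InitStatusData to fill in.
; On BeginPlay it caches its owning Pawn and BP_GS_CharacterStatus game state, binds to turn updates and broadcasts OnStatusStart.
; Each turn update decrements LifeTime, but reaching zero triggers nothing here.
; EventStatusEnd broadcasts OnStatusEnd and destroys the actor; EventStatusBegin is empty.
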(event Custom|OnUpdateTurnNumber
  (params (TurnNumber :type Integer))
  (bind _output_get (Variables|Default|SetLife%20Time (- (Variables|Default|GetLife%20Time) 1)))
  (if (<= _output_get 0)
    _))

(event Custom|EventStatusBegin)

(event Custom|EventStatusEnd
  (Default|CallOnStatusEnd self)
  (Actor|DestroyActor))

(event EventBeginPlay
  (CallFunction|InitStatusData)
  (bind _bsuccess_ (CallFunction|InitCasts))
  (if _bsuccess_
    (EventDispatchers|BindEventtoOnUpdateTurnNumber (Variables|Default|GetAs%20BP%20GS%20Character%20Status) (EventDispatchers|CreateEvent :!event Custom|OnUpdateTurnNumber))
    (Default|CallOnStatusStart self)))

(event Collision|EventActorBeginOverlap
  (params (OtherActor :type Actor%20Object%20Reference)))

(event EventTick
  (params (DeltaSeconds :type Float%20%28single-precision%29)))

(fn ConstructionScript)

(fn InitStatusData)

(fn InitCasts
  (bind _aspawn (Utilities|Casting|CastToPawn (Components|GetOwner))
    (:then
      (Variables|Default|SetAs%20Owning%20%20Pawn _aspawn)
      (bind _asbp_gs_character_status (Utilities|Casting|CastToBP_GS_CharacterStatus (Game|GetGameState))
        (:then
          (Variables|Default|SetAs%20BP%20GS%20Character%20Status _asbp_gs_character_status)
          (return true))
        (:CastFailed
          (return false))))
    (:CastFailed
      (return false))))