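; Kinematic character status actor that sends its owning pawn toward a point on a spline path.
; On status begin, it uses AI Move To toward the world location of the spline point at the current path index.
; Success increments the index without issuing another move, while failure ends the status.
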(event EventBeginPlay
  (|CallParentFunction) ; This node is disabled and will not be called.\nDrag off pins to build functionality.
)

(event Collision|EventActorBeginOverlap
  (params (OtherActor :type Actor%20Object%20Reference))
  (|CallParentFunction OtherActor) ; This node is disabled and will not be called.\nDrag off pins to build functionality.
)

(event EventTick
  (params (DeltaSeconds :type Float%20%28single-precision%29))
  (|CallParentFunction DeltaSeconds) ; This node is disabled and will not be called.\nDrag off pins to build functionality.
)

(event EventEventStatusBegin
  (|CallParentFunction)
  (bind _as_owning__pawn (Variables|Default|GetAs%20Owning%20%20Pawn)
    (:then
      (bind _location (CallFunction|GetSplinePointWorldLocationatIndex (Variables|Default|GetPathPointIndex)))
      (AI|AIMoveTo _as_owning__pawn _location 0 5.0 false
        (:OnSuccess
          (Variables|Default|SetPathPointIndex (+ (Variables|Default|GetPathPointIndex) 1)))
        (:OnFail
          (CallFunction|EventStatusEnd))))
    (:else)))

(event EventEventStatusEnd
  (|CallParentFunction))

(fn ConstructionScript
  (|CallParentFunction))

(fn GetSplinePointWorldLocationatIndex
  (params (PointIndex :type Integer))
  (return (Spline|GetLocationatSplinePoint (Variables|Default|GetSpline) PointIndex "World")))