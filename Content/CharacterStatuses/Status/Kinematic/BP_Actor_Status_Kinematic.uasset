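; Kinematic status actor that moves its owning pawn by AI MoveTo to a target actor or location, ending the status on success or failure.
; When the move starts, it copies the navigation path into a spline, detaches itself and opens a Tick gate.
; Each tick it stops movement if the spline distance at the mouse cursor's hit, not the pawn, reaches MaxMoveDistance.
; Debug prints and points remain; manual spline-following code is disconnected.
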(event Custom|StartCountingSteps
  (Variables|Default|SetPreviousParentLocation (Transformation|GetActorLocation (Variables|Default|GetAs%20Owning%20%20Pawn)))
  (CallFunction|GeneratePathSpline)
  (Variables|Default|SetCurrentWalkDistance 0.0)
  (Utilities|FlowControl|Gate true) ; enters at Open
)

(event Custom|StopCountingSteps
  (Utilities|FlowControl|Gate true) ; enters at Close
)

(event EventBeginPlay
  (|CallParentFunction) ; This node is disabled and will not be called.\nDrag off pins to build functionality.
)

(event Collision|EventActorBeginOverlap
  (params (OtherActor :type Actor%20Object%20Reference))
  (|CallParentFunction OtherActor) ; This node is disabled and will not be called.\nDrag off pins to build functionality.
)

(event EventTick
  (params (DeltaSeconds :type Float%20%28single-precision%29))
  (|CallParentFunction DeltaSeconds)
  (Utilities|FlowControl|Gate true
    (:Exit
      (CallFunction|CalculateSteps))))

(event EventEventStatusBegin
  (Variables|Default|GetAs%20Owning%20%20Pawn
    (:then
      (Variables|Default|GetTarget%20Actor
        (:then
          (AI|AIMoveTo (Variables|Default|GetAs%20Owning%20%20Pawn) "0, 0, 0" (Variables|Default|GetTarget%20Actor) 5.0 false
            (:then
              (CallFunction|StartCountingSteps))
            (:OnSuccess
              (CallFunction|StopCountingSteps :!label _label)
              (CallFunction|EventStatusEnd))
            (:OnFail
              (goto _label))))
        (:else
          (AI|AIMoveTo (Variables|Default|GetAs%20Owning%20%20Pawn) (Variables|Default|GetTargetLocation) 0 5.0 false
            (:then
              (CallFunction|StartCountingSteps))
            (:OnSuccess
              (CallFunction|StopCountingSteps :!label _label_2)
              (CallFunction|EventStatusEnd))
            (:OnFail
              (goto _label_2))))))
    (:else)))

(fn ConstructionScript
  (|CallParentFunction))

(fn SetMovementSpeed)

(fn CalculateSteps
  (bind _returnvalue (Game|GetPlayerController 0))
  (bind _spline (Variables|Default|GetSpline))
  (bind _hitresult (Game|Player|GetHitResultUnderCursorbyChannel _returnvalue "TraceTypeQuery1" true))
  (bind _returnvalue_2 (Class|SplineComponent|GetDistanceAlongSplineatLocation _spline (.location _hitresult) "World"))
  (bind _as_owning__pawn (Variables|Default|GetAs%20Owning%20%20Pawn)
    (:then
      (Development|PrintString (Utilities|String|ToString(Float) _returnvalue_2))
      (if (>= _returnvalue_2 (Variables|Default|GetMaxMoveDistance))
        (AI|Navigation|StopMovement (AI|GetAIController (Variables|Default|GetAs%20Owning%20%20Pawn)))))
    (:else)))

(fn GeneratePathSpline
  (bind _as_owning__pawn (Variables|Default|GetAs%20Owning%20%20Pawn))
  (for _array_element (Variables|/Script/NavigationSystem.NavigationPath|GetPathPoints (Class|AIBlueprintHelperLibrary|GetCurrentPath (AI|GetAIController _as_owning__pawn)))
    (Class|SplineComponent|AddPoint (Variables|Default|GetSpline) (Utilities|Struct|MakeSplinePoint 0.0 (Math|Transform|InverseTransformLocation (Transformation|GetActorTransform _as_owning__pawn) _array_element) "0.000000,0.000000,0.000000" "0.000000,0.000000,0.000000" "0.000000,0.000000,0.000000" "1.000000,1.000000,1.000000" "Linear") true)
    (Rendering|Debug|DrawDebugPoint _array_element 1e+01 "(R=1.000000,G=0.000000,B=0.526237,A=1.000000)" 1e+02)
    (Transformation|DetachFromActor "KeepWorld" "KeepWorld" "KeepWorld")))