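; BP_AC_Status is an actor component that holds the collection of statuses active on its owner, likely a character.
; It exposes functions to get all statuses, add one or remove one.
; Adding is gated by a check that rejects a status if any entry in its data's PreventingStatus list is already held.
; It only does bookkeeping, with no active tick logic and no status effects applied here.
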(event EventBeginPlay)

(event EventTick
  (params (DeltaSeconds :type Float%20%28single-precision%29)))

(fn GetAllStatuses
  (return (Variables|Default|GetStatuses)))

(fn AddStatus
  (params (StatusToAdd :type BP%20Actor%20Status%20Object%20Reference))
  (bind (_statustoadd _canadd_) (CallFunction|CanAddStatus? StatusToAdd))
  (if _canadd_
    (Utilities|Array|Add (Variables|Default|GetStatuses) _statustoadd)
    (return)))

(fn RemoveStatus
  (params (StatusToRemove :type BP%20Actor%20Status%20Object%20Reference))
  (bind _returnvalue (Utilities|Array|RemoveItem (Variables|Default|GetStatuses) StatusToRemove))
  (if _returnvalue
    (return)))

(fn CanAddStatus?
  (params (StatusToCheck :type BP%20Actor%20Status%20Object%20Reference))
  (for _array_element (Variables|/Game/CharacterStatuses/Status/Data/PDA_Status.PDA_Status_C|GetPreventingStatus (Variables|/Game/CharacterStatuses/Status/BP_Actor_Status.BP_Actor_Status_C|GetStatusData StatusToCheck))
    (if (Utilities|Array|ContainsItem (Variables|Default|GetStatuses) _array_element)
      (return 0 false)))
  (return 0 true))