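; Stealth status actor that hides the owning character from the local player when their teams differ.
; On status begin, it compares the character's team with player state 0's team and sets the pawn hidden in game on a mismatch, leaving teammates visible.
; The check runs only at status begin, and status end always unhides the pawn.
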(event EventBeginPlay
  (|CallParentFunction) ; This node is disabled and will not be called.\nDrag off pins to build functionality.
)

(event Collision|EventActorBeginOverlap
  (params (OtherActor :type Actor%20Object%20Reference))
  (|CallParentFunction OtherActor) ; This node is disabled and will not be called.\nDrag off pins to build functionality.
)

(event EventTick
  (params (DeltaSeconds :type Float%20%28single-precision%29))
  (|CallParentFunction DeltaSeconds) ; This node is disabled and will not be called.\nDrag off pins to build functionality.
)

(event EventEventStatusBegin
  (bind _as_owning__pawn (Variables|Default|GetAs%20Owning%20%20Pawn))
  (|CallParentFunction)
  (bind _asbp_character_character_status (Utilities|Casting|CastToBP_Character_CharacterStatus _as_owning__pawn))
  (Rendering|SetActorHiddenInGame _as_owning__pawn (Utilities|Enum|NotEqual(Enum) (Variables|/Game/CharacterStatuses/Character/BP_Character_CharacterStatus.BP_Character_CharacterStatus_C|GetTeam _asbp_character_character_status) (Variables|/Game/CharacterStatuses/Player/State/BP_PS_CharacterStatus.BP_PS_CharacterStatus_C|GetTeam (.AsBP%20PS%20Character%20Status (Utilities|Casting|CastToBP_PS_CharacterStatus (Game|GetPlayerState 0)))))))

(event EventEventStatusEnd
  (|CallParentFunction)
  (Rendering|SetActorHiddenInGame (Variables|Default|GetAs%20Owning%20%20Pawn) false))

(fn ConstructionScript
  (|CallParentFunction))