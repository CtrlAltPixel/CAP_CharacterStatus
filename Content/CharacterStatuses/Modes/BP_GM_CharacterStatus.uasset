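; Game mode for the CharacterStatus mode, providing an event to spawn a player character for a given player controller.
; SpawnCharacter creates BP_Character_CharacterStatus_Player with that controller as its CommandController, then tells the controller's BP_Pawn_Camera to focus on it.
; PostLogin and OnLogout are empty; logic that registers new players and spawns them at a random PlayerStart is disconnected and never runs.
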(event Custom|SpawnCharacter
  (params (SpawnTransform :type Transform) (PlayerController :type Player%20Controller%20Object%20Reference))
  (bind _returnvalue (Game|SpawnActorfromClass "/Game/CharacterStatuses/Character/Player/BP_Character_CharacterStatus_Player.BP_Character_CharacterStatus_Player_C" SpawnTransform "Undefined" "MultiplyWithRoot" 0 PlayerController 0 "NewEnumerator0" 0))
  (bind _asbp_pawn_camera (Utilities|Casting|CastToBP_Pawn_Camera (Pawn|GetControlledPawn PlayerController)))
  (Default|CameraFocus _asbp_pawn_camera _returnvalue))

(event EventBeginPlay)

(event EventTick
  (params (DeltaSeconds :type Float%20%28single-precision%29)))

(event EventPostLogin
  (params (NewPlayer :type Player%20Controller%20Object%20Reference)))

(event EventOnLogout
  (params (ExitingController :type Controller%20Object%20Reference)))

(fn ConstructionScript)