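; Game State for a turn-based character status test mode, running turns until a turn limit ends the match.
; Each turn steps through timed player planning, then Spells, Preparation, Dash, Combat, Deaths and Movement resolution.
; Planning and Spells update player controller states, while each resolve phase begins BP_Actor_Status actors with a matching activation phase.
; RepNotifies broadcast turn and phase changes; Spells resolution and phase end sit inside the per-player loop.
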(event Custom|EventTurnStart
  ;[0.15 0.15 0.15 0.5] Comment
  (Development|PrintString "GS - TurnStart" true true "(R=0.000000,G=0.660000,B=1.000000,A=1.000000)" 3.0)
  (CallFunction|UpdateTurnCount)
  (Variables|Default|SetPhase "NewEnumerator0")
  (CallFunction|EventPhaseStart))

(event Custom|EventTurnEnd
  ;[0.15 0.15 0.15 0.5] Comment
  (Development|PrintString "GS - Turn End" true true "(R=0.000000,G=0.660000,B=1.000000,A=1.000000)" 3.0)
  (bind _bismaxscore_ (CallFunction|IsMaxTurn?))
  (if _bismaxscore_
    (Development|PrintString "GS - Match End")
    (else
      (CallFunction|EventTurnStart))))

(event Custom|EventPhaseEnd
  ;[0.15 0.15 0.15 0.5] Comment
  (Development|PrintString "GS - PhaseEnd" true true "(R=0.000000,G=0.660000,B=1.000000,A=1.000000)" 3.0)
  (switch Utilities|FlowControl|Switch|SwitchonE_Phase (Variables|Default|GetPhase)
    (:NewEnumerator0
      (Variables|Default|SetPhase "NewEnumerator1")
      (CallFunction|EventPhaseStart :!label _label))
    (:NewEnumerator1
      (Variables|Default|SetPhase "NewEnumerator2")
      (goto _label))
    (:NewEnumerator2
      (Variables|Default|SetPhase "NewEnumerator3")
      (goto _label))
    (:NewEnumerator3
      (Variables|Default|SetPhase "NewEnumerator4")
      (goto _label))
    (:NewEnumerator4
      (Variables|Default|SetPhase "NewEnumerator5")
      (goto _label))
    (:NewEnumerator5
      (Variables|Default|SetPhase "NewEnumerator6")
      (goto _label))
    (:NewEnumerator6
      (Variables|Default|SetPhase "NewEnumerator0")
      (CallFunction|EventTurnEnd))))

(event Custom|EventPhaseStart
  ;[0.15 0.15 0.15 0.5] Comment
  (Utilities|FlowControl|Delay 1.0)
  (switch Utilities|FlowControl|Switch|SwitchonE_Phase (Variables|Default|GetPhase)
    (:NewEnumerator0
      (Development|PrintString "GS - PhaseStart (Player Planning)" true true "(R=0.000000,G=0.660000,B=1.000000,A=1.000000)" 3.0)
      (bind _returnvalue (Utilities|Time|SetTimerbyEvent (EventDispatchers|CreateEvent :!event Custom|EventPhaseEnd) 5.0))
      (bind _output_get (Variables|Default|SetPhaseTimer _returnvalue))
      (Development|PrintString (Utilities|String|Append "GS - " (Utilities|String|ToString(Float) (Utilities|Time|GetTimerRemainingTimebyHandle _output_get)) "s Remaining!") true true "(R=0.000000,G=0.660000,B=1.000000,A=1.000000)" 3.0)
      (for _array_element (Variables|Default|GetPlayerArray)
        (bind _asbp_pc_character_status (Utilities|Casting|CastToBP_PC_CharacterStatus (Game|GetPlayerController _array_element)))
        (Default|UpdatePlayerState _asbp_pc_character_status "NewEnumerator4")))
    (:NewEnumerator1
      (Development|PrintString "GS - PhaseStart (Resolving Spells)" true true "(R=0.000000,G=0.660000,B=1.000000,A=1.000000)" 3.0)
      (Utilities|Time|InvalidateTimerHandle (Variables|Default|GetPhaseTimer))
      (for _array_element_2 (Variables|Default|GetPlayerArray)
        (bind _asbp_pc_character_status_2 (Utilities|Casting|CastToBP_PC_CharacterStatus (Game|GetPlayerController _array_element_2)))
        (Default|UpdatePlayerState _asbp_pc_character_status_2 "NewEnumerator3")
        (bind _outactors (Actor|GetAllActorsOfClass "/Game/CharacterStatuses/Status/BP_Actor_Status.BP_Actor_Status_C"))
        (for _array_element_3 _outactors
          (if (Utilities|Enum|Equal(Enum) (Variables|Default|GetPhase) (Variables|/Game/CharacterStatuses/Status/BP_Actor_Status.BP_Actor_Status_C|GetActivationPhase _array_element_3))
            (Default|EventStatusBegin _array_element_3)))
        (CallFunction|EventPhaseEnd)))
    (:NewEnumerator2
      (Development|PrintString "GS - PhaseStart (Resolving Preperation)" true true "(R=0.000000,G=1.000000,B=0.000000,A=1.000000)" 3.0)
      (bind _outactors_2 (Actor|GetAllActorsOfClass "/Game/CharacterStatuses/Status/BP_Actor_Status.BP_Actor_Status_C"))
      (for _array_element_4 _outactors_2
        (if (Utilities|Enum|Equal(Enum) (Variables|Default|GetPhase) (Variables|/Game/CharacterStatuses/Status/BP_Actor_Status.BP_Actor_Status_C|GetActivationPhase _array_element_4))
          (Default|EventStatusBegin _array_element_4)))
      (CallFunction|EventPhaseEnd))
    (:NewEnumerator3
      (Development|PrintString "GS - PhaseStart (Resolving Dash)" true true "(R=1.000000,G=1.000000,B=0.000000,A=1.000000)" 3.0)
      (bind _outactors_3 (Actor|GetAllActorsOfClass "/Game/CharacterStatuses/Status/BP_Actor_Status.BP_Actor_Status_C"))
      (for _array_element_5 _outactors_3
        (if (Utilities|Enum|Equal(Enum) (Variables|Default|GetPhase) (Variables|/Game/CharacterStatuses/Status/BP_Actor_Status.BP_Actor_Status_C|GetActivationPhase _array_element_5))
          (Default|EventStatusBegin _array_element_5)))
      (CallFunction|EventPhaseEnd))
    (:NewEnumerator4
      (Development|PrintString "GS - PhaseStart (Resolving Combat)" true true "(R=1.000000,G=0.000000,B=0.000000,A=1.000000)" 3.0)
      (bind _outactors_4 (Actor|GetAllActorsOfClass "/Game/CharacterStatuses/Status/BP_Actor_Status.BP_Actor_Status_C"))
      (for _array_element_6 _outactors_4
        (if (Utilities|Enum|Equal(Enum) (Variables|Default|GetPhase) (Variables|/Game/CharacterStatuses/Status/BP_Actor_Status.BP_Actor_Status_C|GetActivationPhase _array_element_6))
          (Default|EventStatusBegin _array_element_6)))
      (CallFunction|EventPhaseEnd))
    (:NewEnumerator5
      (Development|PrintString "GS - PhaseStart (Resolving Death)" true true "(R=0.000000,G=0.660000,B=1.000000,A=1.000000)" 3.0)
      (bind _outactors_5 (Actor|GetAllActorsOfClass "/Game/CharacterStatuses/Status/BP_Actor_Status.BP_Actor_Status_C"))
      (for _array_element_7 _outactors_5
        (if (Utilities|Enum|Equal(Enum) (Variables|Default|GetPhase) (Variables|/Game/CharacterStatuses/Status/BP_Actor_Status.BP_Actor_Status_C|GetActivationPhase _array_element_7))
          (Default|EventStatusBegin _array_element_7)))
      (CallFunction|EventPhaseEnd))
    (:NewEnumerator6
      (Development|PrintString "GS - PhaseStart (Resolving Movement)" true true "(R=0.041667,G=0.041667,B=0.041667,A=1.000000)" 3.0)
      (bind _outactors_6 (Actor|GetAllActorsOfClass "/Game/CharacterStatuses/Status/BP_Actor_Status.BP_Actor_Status_C"))
      (for _array_element_8 _outactors_6
        (if (Utilities|Enum|Equal(Enum) (Variables|Default|GetPhase) (Variables|/Game/CharacterStatuses/Status/BP_Actor_Status.BP_Actor_Status_C|GetActivationPhase _array_element_8))
          (Default|EventStatusBegin _array_element_8)))
      (CallFunction|EventPhaseEnd))))

(event EventBeginPlay
  ;[0.15 0.15 0.15 0.5] Comment
  (Utilities|Time|SetTimerbyEvent (EventDispatchers|CreateEvent :!event Custom|EventTurnStart) 3.0))

(event EventTick
  (params (DeltaSeconds :type Float%20%28single-precision%29)))

(fn ConstructionScript)

(fn OnRepCurrentTurnNumber
  (Default|CallOnUpdateTurnNumber (Variables|Default|GetCurrentTurnNumber)))

(fn OnRepPhase
  (Default|CallOnPhaseStart (Variables|Default|GetPhase)))

(fn IsMaxTurn?
  (return (== (Variables|Default|GetCurrentTurnNumber) 20)))

(fn UpdateTurnCount
  (Variables|Default|SetCurrentTurnNumber (+ (Variables|Default|GetCurrentTurnNumber) 1)))