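; Player controller for the CharacterStatus setup that drives a camera pawn, selects characters under the cursor and toggles the HUD's dead overlay from player state.
; On local BeginPlay it adds camera and interact Enhanced Input contexts, caches HUD and pawn, and enables mouse events.
; Interact traces under the cursor, temporarily adding a drag context when nothing is hit.
; A debug key spawns and applies a kinematic status to the selected character.
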(event Custom|UpdatePlayerState
  (params (PlayerState :type E_PlayerState%20Enum :default "NewEnumerator0"))
  ;[0.15 0.15 0.15 0.5] Comment
  (bind _output_get (Variables|Default|SetPlayer%20State PlayerState))
  (switch Utilities|FlowControl|Switch|SwitchonE_PlayerState _output_get
    (:NewEnumerator1
      (bind _as_bp_hud_character_status (Variables|Default|GetAs%20BP%20HUD%20Character%20Status)
        (:then
          (Default|ToggleDeadOverlay _as_bp_hud_character_status "Collapsed"))
        (:else)))
    (:NewEnumerator2
      (bind _as_bp_hud_character_status_2 (Variables|Default|GetAs%20BP%20HUD%20Character%20Status)
        (:then
          (Default|ToggleDeadOverlay _as_bp_hud_character_status_2 "HitTestInvisible"))
        (:else)))))

(event Input|EnhancedActionEvents|EnhancedInputActionIA_CameraMove
  (params (ActionValue :type Vector%202D%20Structure) (ElapsedSeconds :type Float%20%28double-precision%29) (TriggeredSeconds :type Float%20%28double-precision%29) (InputAction :type Input%20Action%20Object%20Reference :default "/Game/CharacterStatuses/Input/Actions/Camera/IA_CameraMove.IA_CameraMove"))
  ;[0.15 0.15 0.15 0.5] Camera
  (bind _as_bp_pawn_camera (Variables|Default|GetAs%20BP%20Pawn%20Camera)
    (:then
      (Default|CameraMove _as_bp_pawn_camera (.x ActionValue) (.y ActionValue)))
    (:else)))

(event Input|EnhancedActionEvents|EnhancedInputActionIA_Interact
  (params (ActionValue :type Boolean) (ElapsedSeconds :type Float%20%28double-precision%29) (TriggeredSeconds :type Float%20%28double-precision%29) (InputAction :type Input%20Action%20Object%20Reference :default "/Game/CharacterStatuses/Input/Actions/IA_Interact.IA_Interact"))
  (bind (_hit_ _hitactor) (CallFunction|GetActorUnderCursorbyChannel "TraceTypeQuery3"))
  ;[0.05098 0.05098 0.05098] Set
  (:Triggered
    (if (Class|GameplayStatics|ObjectIsA (Variables|Default|GetAsInteractActor) "/Game/CharacterStatuses/Character/BP_Character_CharacterStatus.BP_Character_CharacterStatus_C")
      (CallFunction|UpdateSelectedCharacter (Variables|Default|GetAsInteractActor))))
  (:Started
    (if _hit_
      (Utilities|IsValid _hitactor
        (:Is%20Valid
          (Variables|Default|SetAsInteractActor _hitactor))
        (:Is%20Not%20Valid
          (Input|AddMappingContext (PlayerController|LocalPlayerSubsystems|GetEnhancedInputLocalPlayerSubsystem) "/Game/CharacterStatuses/Input/IMC_Drag.IMC_Drag" 0 "(bIgnoreAllPressedKeysUntilRelease=True,bForceImmediately=False,bNotifyUserSettings=False)" :!label _label)))
      (else
        (goto _label))))
  (:Canceled
    (Input|RemoveMappingContext (PlayerController|LocalPlayerSubsystems|GetEnhancedInputLocalPlayerSubsystem) "/Game/CharacterStatuses/Input/IMC_Drag.IMC_Drag" "(bIgnoreAllPressedKeysUntilRelease=True,bForceImmediately=False,bNotifyUserSettings=False)" :!label _label_2))
  (:Completed
    (goto _label_2)))

(event Input|EnhancedActionEvents|EnhancedInputActionIA_CameraReset
  (params (ActionValue :type Boolean) (ElapsedSeconds :type Float%20%28double-precision%29) (TriggeredSeconds :type Float%20%28double-precision%29) (InputAction :type Input%20Action%20Object%20Reference :default "/Game/CharacterStatuses/Input/Actions/Camera/IA_CameraReset.IA_CameraReset"))
  ;[0.15 0.15 0.15 0.5] Camera
  (bind _as_bp_pawn_camera (Variables|Default|GetAs%20BP%20Pawn%20Camera)
    (:then
      (Default|CameraFocus _as_bp_pawn_camera (Variables|Default|GetAs%20BP%20Character%20Character%20Status)))
    (:else)))

(event Input|EnhancedActionEvents|EnhancedInputActionIA_Drag
  (params (ActionValue :type Vector%202D%20Structure) (ElapsedSeconds :type Float%20%28double-precision%29) (TriggeredSeconds :type Float%20%28double-precision%29) (InputAction :type Input%20Action%20Object%20Reference :default "/Game/CharacterStatuses/Input/Actions/Drag/IA_Drag.IA_Drag"))
  ;[0.15 0.15 0.15 0.5] Comment
  (bind _as_bp_pawn_camera (Variables|Default|GetAs%20BP%20Pawn%20Camera)
    (:then
      (Default|CameraDrag _as_bp_pawn_camera (.x ActionValue) (.y ActionValue)))
    (:else)))

(event EventBeginPlay
  (bind _returnvalue (PlayerController|LocalPlayerSubsystems|GetEnhancedInputLocalPlayerSubsystem))
  ;[0.05098 0.05098 0.05098] Add Mapping Context
  (if (Pawn|IsLocalPlayerController)
    (Utilities|IsValid _returnvalue
      (:Is%20Valid
        (Input|AddMappingContext _returnvalue "/Game/CharacterStatuses/Input/IMC_Camera.IMC_Camera" 0 "(bIgnoreAllPressedKeysUntilRelease=True,bForceImmediately=False,bNotifyUserSettings=False)")
        (Input|AddMappingContext _returnvalue "/Game/CharacterStatuses/Input/IMC_Interact.IMC_Interact" 0 "(bIgnoreAllPressedKeysUntilRelease=True,bForceImmediately=False,bNotifyUserSettings=False)")
        (CallFunction|InitCasts)
        (Variables|Default|SetCurrentClickTraceChannel "ECC_GameTraceChannel1")
        (Variables|Default|SetbShowMouseCursor true)
        (Variables|Default|SetbEnableClickEvents true)
        (Variables|Default|SetbEnableMouseOverEvents true)))))

(event Input|KeyboardEvents|DebugKey1
  (params (Key :type Key%20Structure :default "None") (ActionValue :type Input%20Action%20Value%20Structure)))

(event Input|KeyboardEvents|DebugKey2
  (params (Key :type Key%20Structure :default "None") (ActionValue :type Input%20Action%20Value%20Structure)))

(event Input|KeyboardEvents|DebugKey3
  (params (Key :type Key%20Structure :default "None") (ActionValue :type Input%20Action%20Value%20Structure)))

(event Input|KeyboardEvents|DebugKey4
  (params (Key :type Key%20Structure :default "None") (ActionValue :type Input%20Action%20Value%20Structure)))

(event Input|KeyboardEvents|DebugKey5
  (params (Key :type Key%20Structure :default "None") (ActionValue :type Input%20Action%20Value%20Structure)))

(event Input|KeyboardEvents|DebugKey6
  (params (Key :type Key%20Structure :default "None") (ActionValue :type Input%20Action%20Value%20Structure)))

(event Input|KeyboardEvents|DebugKey7
  (params (Key :type Key%20Structure :default "None") (ActionValue :type Input%20Action%20Value%20Structure)))

(event Input|KeyboardEvents|DebugKey8
  (params (Key :type Key%20Structure :default "None") (ActionValue :type Input%20Action%20Value%20Structure))
  (bind _as_bp_character_character_status (Variables|Default|GetAs%20BP%20Character%20Character%20Status))
  (:Pressed
    (bind _returnvalue (Game|SpawnActorfromClass "/Game/CharacterStatuses/Status/Kinematic/BP_Actor_Status_Kinematic.BP_Actor_Status_Kinematic_C" (Transformation|GetActorTransform _as_bp_character_character_status) "AlwaysSpawn" "MultiplyWithRoot" _as_bp_character_character_status (+ (Transformation|GetActorLocation _as_bp_character_character_status) "0.000000,500.000000,0.000000") 0 5e+02 0))
    (Default|AddStatus (Variables|/Game/CharacterStatuses/Character/BP_Character_CharacterStatus.BP_Character_CharacterStatus_C|GetBP_AC_Status (Variables|Default|GetAs%20BP%20Character%20Character%20Status)) _returnvalue)))

(event Input|KeyboardEvents|DebugKey9
  (params (Key :type Key%20Structure :default "None") (ActionValue :type Input%20Action%20Value%20Structure)))

(fn ConstructionScript)

(fn GetActorUnderCursorbyChannel
  (params (TraceChannel :type ETraceTypeQuery%20Enum :default "TraceTypeQuery1"))
  (bind _hitresult (Game|Player|GetHitResultUnderCursorbyChannel TraceChannel true))
  (bind (_bblockinghit _binitialoverlap _time _distance _location _impactpoint _normal _impactnormal _physmat _hitactor) (Collision|BreakHitResult _hitresult))
  (return _bblockinghit _hitactor))

(fn UpdateSelectedCharacter
  (params (Actor :type Actor%20Object%20Reference))
  (bind _asbp_character_character_status (Utilities|Casting|CastToBP_Character_CharacterStatus Actor))
  (Variables|Default|SetAs%20BP%20Character%20Character%20Status _asbp_character_character_status))

(fn InitCasts
  (bind _asbp_hud_character_status (Utilities|Casting|CastToBP_HUD_CharacterStatus (HUD|GetHUD))
    (:then
      (Variables|Default|SetAs%20BP%20HUD%20Character%20Status _asbp_hud_character_status)
      (bind _asbp_pawn_camera (Utilities|Casting|CastToBP_Pawn_Camera (Pawn|GetControlledPawn))
        (:then
          (Variables|Default|SetAs%20BP%20Pawn%20Camera _asbp_pawn_camera)
          (return true))
        (:CastFailed
          (return false))))
    (:CastFailed
      (return false))))