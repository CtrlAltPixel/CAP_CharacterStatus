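; Actor component that holds a character's replicated attributes, such as Health, Resource, resists and Haste, with empty RepNotify handlers.
; UpdateAttribute adds a value to the chosen struct field, then calls the update dispatcher.
; Owner damage adds the unnegated Damage value to current Health through that function.
; A second after BeginPlay, it attaches a screen-space HUD widget above the owner's bounds.
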(event Custom|EventSpawnUI
  (bind _returnvalue (Components|GetOwner))
  (Utilities|IsValid _returnvalue
    (:Is%20Valid
      (bind _returnvalue_2 (UserInterface|CreateWidget "/Game/CharacterStatuses/Attributes/UI/WB_Attributes_CharacterHUD.WB_Attributes_CharacterHUD_C" 0 _returnvalue))
      (Variables|Default|SetAsWBAttributesHUD _returnvalue_2)
      (bind _returnvalue_3 (Game|AddComponentbyClass _returnvalue "/Script/UMG.WidgetComponent" false (Math|Transform|MakeTransform (Math|Vector|MakeVector 0.0 0.0 (+ (.z (.BoxExtent (Collision|GetActorBounds _returnvalue true false))) 1e+01)) "0, 0, 0" "1.000000,1.000000,1.000000")))
      (Variables|Default|SetWidgetComponent _returnvalue_3)
      (UserInterface|SetWidget _returnvalue_3 (Variables|Default|GetAsWBAttributesHUD))
      (Class|WidgetComponent|SetWidgetSpace _returnvalue_3 "Screen")
      (Class|WidgetComponent|SetDrawatDesiredSize _returnvalue_3 true)
      (Default|AttributeUpdated (Variables|Default|GetAsWBAttributesHUD))
      (Default|SetOwnerOfBars (Variables|Default|GetAsWBAttributesHUD) (Components|GetOwner)))))

(event Custom|CalculateDamage
  (params (DamagedActor :type Actor%20Object%20Reference) (Damage :type Float%20%28single-precision%29) (DamageType :type Damage%20Type%20Object%20Reference) (InstigatedBy :type Controller%20Object%20Reference) (DamageCauser :type Actor%20Object%20Reference))
  (CallFunction|UpdateAttribute "NewEnumerator2" (Variables|Default|GetHealth) Damage)
  (Variables|Default|GetAsWBAttributesHUD
    (:then)
    (:else)))

(event EventBeginPlay
  (EventDispatchers|BindEventtoOnTakeAnyDamage (Components|GetOwner) (EventDispatchers|CreateEvent :!event Custom|CalculateDamage))
  (Utilities|FlowControl|Delay 1.0)
  (CallFunction|EventSpawnUI))

(event EventTick
  (params (DeltaSeconds :type Float%20%28single-precision%29)))

(fn GetAttribute
  (params (Index :type E_Attributes_Name%20Enum :default "NewEnumerator0"))
  (return (Utilities|Array|Get(acopy) (Utilities|Array|MakeArray (Variables|Default|GetHealth) (Variables|Default|GetResource) (Variables|Default|GetMagicResist) (Variables|Default|GetSpellShield) (Variables|Default|GetPhysicalResist) (Variables|Default|GetArmour) (Variables|Default|GetHaste)) (Math|Conversions|ToInteger(Byte) Index))))

(fn CalculateAttribute
  (params (Attribute :type F%20Attributes%20Structure%20%28by%20ref%29))
  (bind (_name _base _bonus _current _max _multiplier) (Utilities|Struct|BreakF_Attributes Attribute))
  (return (* (+ _base _bonus) _multiplier)))

(fn UpdateAttribute
  (params (AttributeType :type E_Attributes_Type%20Enum :default "NewEnumerator0") (Attribute :type F%20Attributes%20Structure%20%28by%20ref%29) (Value :type Float%20%28double-precision%29%20%28by%20ref%29))
  (Utilities|FlowControl|Sequence
    (:then_0
      (switch Utilities|FlowControl|Switch|SwitchonE_Attributes_Type AttributeType
        (:NewEnumerator0
          (Private|ModifyAttributeBase Attribute Value))
        (:NewEnumerator1
          (Private|ModifyAttributeBonus Attribute Value))
        (:NewEnumerator2
          (Private|ModifyAttributeCurrent Attribute Value))
        (:NewEnumerator3
          (Private|ModifyAttributeMax Attribute Value))
        (:NewEnumerator4
          (Private|ModifyAttributeMultiplier Attribute Value))
        (:NewEnumerator5
          (Private|ModifyAttributeRegen Attribute Value))))
    (:then_1
      (Default|CallOnUpdateAttribute Attribute))))

(fn ModifyAttributeBase
  (params (AttributeData :type F%20Attributes%20Structure%20%28by%20ref%29) (Value :type Float%20%28double-precision%29))
  (bind _structout (Utilities|Struct|SetmembersinF_Attributes AttributeData (+ (.Base (Utilities|Struct|BreakF_Attributes AttributeData)) Value)))
  (return _structout))

(fn ModifyAttributeBonus
  (params (AttributeData :type F%20Attributes%20Structure%20%28by%20ref%29) (Value :type Float%20%28double-precision%29))
  (bind _structout (Utilities|Struct|SetmembersinF_Attributes AttributeData (+ (.Bonus (Utilities|Struct|BreakF_Attributes AttributeData)) Value)))
  (return _structout))

(fn ModifyAttributeCurrent
  (params (AttributeData :type F%20Attributes%20Structure%20%28by%20ref%29) (Value :type Float%20%28double-precision%29))
  (bind _structout (Utilities|Struct|SetmembersinF_Attributes AttributeData (+ (.Current (Utilities|Struct|BreakF_Attributes AttributeData)) Value)))
  (return _structout))

(fn ModifyAttributeMax
  (params (AttributeData :type F%20Attributes%20Structure%20%28by%20ref%29) (Value :type Float%20%28double-precision%29))
  (bind _structout (Utilities|Struct|SetmembersinF_Attributes AttributeData (+ (.Max (Utilities|Struct|BreakF_Attributes AttributeData)) Value)))
  (return _structout))

(fn ModifyAttributeMultiplier
  (params (AttributeData :type F%20Attributes%20Structure%20%28by%20ref%29) (Value :type Float%20%28double-precision%29))
  (bind _structout (Utilities|Struct|SetmembersinF_Attributes AttributeData (+ (.Multiplier (Utilities|Struct|BreakF_Attributes AttributeData)) Value)))
  (return _structout))

(fn ModifyAttributeRegen
  (params (AttributeData :type F%20Attributes%20Structure%20%28by%20ref%29) (Value :type Float%20%28double-precision%29))
  (bind _structout (Utilities|Struct|SetmembersinF_Attributes AttributeData (+ (.Regen (Utilities|Struct|BreakF_Attributes AttributeData)) Value)))
  (return _structout))

(fn OnRepHealth)

(fn OnRepResource)

(fn OnRepMagicResist)

(fn OnRepSpellShield)

(fn OnRepPhysicalResist)

(fn OnRepArmour)

(fn OnRepHaste)