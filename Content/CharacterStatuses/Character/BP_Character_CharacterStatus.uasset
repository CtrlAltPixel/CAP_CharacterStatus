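; Character Blueprint with hover and interaction feedback, set up to use the CharacterStatus AI controller.
; On BeginPlay it creates dynamic materials for a cyan outline and an interact decal, blocks a custom trace channel on the capsule and assigns the controller class.
; Cursor over/out toggles the outline through the mesh's overlay material.
; Begin/End interact events show or hide the decal, which the mesh itself does not receive.
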(event Custom|BeginActorInteract
  (Rendering|SetVisibility (Variables|Default|GetDecal_Interact) true false))

(event Custom|EndActorInteract
  (Rendering|SetVisibility (Variables|Default|GetDecal_Interact) false false))

(event EventBeginPlay
  (CallFunction|InitMatDecalOverlay)
  (CallFunction|InitMaterialInteract)
  (CallFunction|InitCharacter))

(event MouseInput|EventActorBeginCursorOver
  (Rendering|Material|SetOverlayMaterial (Variables|Character|GetMesh) (Variables|Default|GetOverlayMaterial) :!class /Script/Engine.MeshComponent))

(event MouseInput|EventActorEndCursorOver
  (Rendering|Material|SetOverlayMaterial (Variables|Character|GetMesh) 0 :!class /Script/Engine.MeshComponent))

(fn ConstructionScript)

(fn InitMatDecalOverlay
  (bind _returnvalue (Rendering|Material|CreateDynamicMaterialInstance "/Game/CharacterStatuses/Character/Material/MAT_OutlineOverlay.MAT_OutlineOverlay" "None" "None" :!class /Script/Engine.KismetMaterialLibrary))
  (bind _output_get (Variables|Default|SetOverlayMaterial _returnvalue))
  (Rendering|Material|SetVectorParameterValue _output_get "Colour" "(R=0.000000,G=1.000000,B=1.000000,A=1.000000)" :!class /Script/Engine.MaterialInstanceDynamic)
  (Rendering|Components|Decal|SetDecalMaterial (Variables|Default|GetDecal_Interact) (Variables|Default|GetMAT_Decal_Interact)))

(fn InitMaterialInteract
  (bind _returnvalue (Rendering|Material|CreateDynamicMaterialInstance "/Game/CharacterStatuses/Character/Material/MAT_Decal_Interact.MAT_Decal_Interact" "None" "None" :!class /Script/Engine.KismetMaterialLibrary))
  (bind _output_get (Variables|Default|SetMAT_Decal_Interact _returnvalue))
  (Rendering|Components|Decal|SetDecalMaterial (Variables|Default|GetDecal_Interact) _output_get))

(fn InitCharacter
  (Collision|SetCollisionResponsetoChannel (Variables|Collision|GetCapsuleComponent) "ECC_GameTraceChannel1" "ECR_Block")
  (Rendering|SetVisibility (Variables|Default|GetDecal_Interact) false false)
  (Rendering|SetReceivesDecals (Variables|Character|GetMesh) false)
  (Variables|Default|SetAIControllerClass "/Game/CharacterStatuses/Character/AI/BP_AIController_CharacterStatus.BP_AIController_CharacterStatus_C"))