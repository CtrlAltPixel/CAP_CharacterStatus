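; BP_Actor_SpawnTile is a spawn tile that appears while the local player is dead.
; It binds to the player controller's state change, showing the mesh and blocking a custom trace channel on Dead, then hiding it and ignoring that channel on Alive.
; On Dead it also iterates characters overlapping its range sphere, but only casts them.
; Interact events are empty stubs, and the interact-colour dynamic material is created but never applied.
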(event Custom|EventBeginInteract)

(event Custom|EventEndInteract)

(event Custom|OnChangePlayerState
  (params (PlayerState :type E_PlayerState%20Enum :default "NewEnumerator0"))
  (switch Utilities|FlowControl|Switch|SwitchonE_PlayerState PlayerState
    (:NewEnumerator1
      (Rendering|SetVisibility (Variables|Default|GetStaticMesh_Tile) false false)
      (Collision|SetCollisionResponsetoChannel (Variables|Default|GetStaticMesh_Tile) "ECC_GameTraceChannel1" "ECR_Ignore"))
    (:NewEnumerator2
      (for _array_element (Collision|GetOverlappingActors (Variables|Default|GetSphereCollision_Range) "/Game/CharacterStatuses/Character/BP_Character_CharacterStatus.BP_Character_CharacterStatus_C" :!class /Script/Engine.PrimitiveComponent)
        (bind _asbp_character_character_status (Utilities|Casting|CastToBP_Character_CharacterStatus _array_element)))
      (Rendering|SetVisibility (Variables|Default|GetStaticMesh_Tile) true false)
      (Collision|SetCollisionResponsetoChannel (Variables|Default|GetStaticMesh_Tile) "ECC_GameTraceChannel1" "ECR_Block"))))

(event EventBeginPlay
  (bind _asbp_gm_character_status (Utilities|Casting|CastToBP_GM_CharacterStatus (Game|GetGameMode)))
  (Variables|Default|SetAs%20BP%20GM%20Character%20Status _asbp_gm_character_status)
  (bind _asbp_pc_character_status (Utilities|Casting|CastToBP_PC_CharacterStatus (Game|GetPlayerController 0)))
  (bind _output_get (Variables|Default|SetAsLocalPlayerController _asbp_pc_character_status))
  (EventDispatchers|BindEventtoOnPlayerStateChanged _output_get (EventDispatchers|CreateEvent :!event Custom|OnChangePlayerState))
  (bind _returnvalue (Rendering|Material|CreateDynamicMaterialInstance "/Game/CharacterStatuses/SpawnTile/Material/MAT_InteractColor.MAT_InteractColor" "None" "None" :!class /Script/Engine.KismetMaterialLibrary))
  (Variables|Default|SetAsMATInteractColour _returnvalue))

(event Collision|EventActorBeginOverlap
  (params (OtherActor :type Actor%20Object%20Reference)))

(event EventTick
  (params (DeltaSeconds :type Float%20%28single-precision%29)))

(fn ConstructionScript)